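; Turn-based battle manager that registers with every BPAvversario and serves as the battle camera view target.
; BattleMode saves the player's position, freezes movement, teleports both fighters to markers and starts HUD-driven turns.
; Attacca lerps the attacker forward and back with timelines, waiting out the move's animation before applying damage.
; Either side reaching zero health calls NormalMode(true), which destroys the enemy and restores exploration, even if the player lost.
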(event `self.ReceiveBeginPlay`
  (bind _asbppersonaggio (cast `/Game/Blueprint/BPPersonaggio` (`GameplayStatics.GetPlayerCharacter` 0)))
  (set `self.Giocatore` _asbppersonaggio)
  (bind _outactors (`GameplayStatics.GetAllActorsOfClass` "/Game/Blueprint/BPAvversario.BPAvversario_C"))
  (for _array_element _outactors
    (set `/Game/Blueprint/BPAvversario.GestBattaglia` self _array_element)))

(event `BattleMode`
  (params (Nemico :type "/Game/Blueprint/BPAvversario Object Reference"))
  (bind _returnvalue (`GameplayStatics.GetPlayerController` 0))
  (set `self.Nemico` Nemico)
  (bind _asbppersonaggio (cast `/Game/Blueprint/BPPersonaggio` (`GameplayStatics.GetPlayerCharacter` 0)))
  (`/Game/Blueprint/BPPersonaggio.Salva Posizione` _asbppersonaggio)
  (`CharacterMovementComponent.DisableMovement` (`Character.CharacterMovement` _asbppersonaggio))
  (`self.DisableInput` _asbppersonaggio null)
  (set `PlayerController.bShowMouseCursor` true _returnvalue)
  (`PlayerController.SetViewTargetWithBlend` _returnvalue self 0.0 "VTBlend_Linear" 0.0 false)
  (`self.SetUpBattaglia`)
  (`self.Turno Giocatore`))

(event `SetUpBattaglia`
  (`SceneComponent.K2_SetWorldLocation` (`Actor.RootComponent` (`self.Giocatore`)) (`SceneComponent.K2_GetComponentLocation` (`Actor.RootComponent` (`self.PosGiocatore`))) false true)
  (`SceneComponent.K2_SetWorldLocation` (`Actor.RootComponent` (`self.Nemico`)) (`SceneComponent.K2_GetComponentLocation` (`Actor.RootComponent` (`self.PosNemico`))) false true)
  (bind _outactors (`GameplayStatics.GetAllActorsOfClass` "/Game/Blueprint/BPAvversario.BPAvversario_C"))
  (for _array_element _outactors
    (`CharacterMovementComponent.DisableMovement` (`Character.CharacterMovement` _array_element))))

(event `Turno Giocatore`
  (bind _asbphud (cast `/Game/HUD/BPHud` (`PlayerController.GetHUD` (`GameplayStatics.GetPlayerController` 0))))
  (`/Game/HUD/BPHud.HudTurnoGiocatore` _asbphud))

(event `Turno Avversario`
  (`/Game/HUD/BPHud.HudTurnoNemico` (stale `Turno Giocatore` _asbphud)))

(event `Attacca`
  (params (ChiAttacca :type "PaperCharacter Object Reference") (Danno :type Integer) (Mossa :type "/Game/Dati/Giocatore/MosseGiocatoreEN Enum" :default "NewEnumerator3"))
  (bind _returnvalue (* Danno -1))
  (bind _nemico (`self.Nemico`))
  (bind _giocatore (`self.Giocatore`))
  (bind _giocatore_2 (`self.Giocatore`))
  (bind _nemico_2 (`self.Nemico`))
  (bind _nemico_3 (`self.Nemico`))
  (bind _giocatore_3 (`self.Giocatore`))
  (bind _skillgiocatore (`/Game/Blueprint/BPPersonaggio.SkillGiocatore` (`self.Giocatore`)))
  (bind (_skillnemicost_posizioneattacco _skillnemicost_posizionenormale _skillnemicost_skill1) (break `/Game/Dati/Nemici/MosseNemicoST` (`/Game/Blueprint/BPAvversario.SkillNemicoST` _nemico)))
  (set `self.MossaGiocatore` Mossa)
  (cast `/Game/Blueprint/BPPersonaggio` ChiAttacca
    (:`then`
      (bind _foundwidgets (`WidgetBlueprintLibrary.GetAllWidgetsOfClass` "/Game/HUD/BPWidgetTurnoGiocatore.BPWidgetTurnoGiocatore_C"))
      (for _array_element _foundwidgets
        (`Widget.RemoveFromParent` _array_element))
      (set `/Game/Blueprint/BPPersonaggio.InBattaglia` true _giocatore)
      (set `/Game/Blueprint/BPPersonaggio.MossaScelta` "NewEnumerator3" _giocatore)
      (bind (_direction _newtrack_5) (`Timeline|Timeline_1` :!via `PlayFromStart`)
        (:`Update`
          (`self.MuoviInPosizione` _newtrack_5 (`self.PosGiocatore`) (`self.PosAttaccoGiocatore`) _giocatore_3))
        (:`Finished`
          (set `/Game/Blueprint/BPPersonaggio.MossaScelta` (`self.MossaGiocatore`) _giocatore_3)
          (`KismetSystemLibrary.Delay` (`PaperFlipbook.GetTotalDuration` (select `/Game/Dati/Giocatore/MosseGiocatoreEN` (`self.MossaGiocatore`) :`NewEnumerator3` (`.Animazione_6_A2D9DE42406F882B081E8284B2054071` (break `/Game/Dati/Giocatore/MossaGiocatore` (break `/Game/Dati/Giocatore/MosseAttualiGiocatoreST` _skillgiocatore))) :`NewEnumerator4` (`.Animazione_6_A2D9DE42406F882B081E8284B2054071` (break `/Game/Dati/Giocatore/MossaGiocatore` (`.PosizioneDifesa_34_D2FF22644A8F68D2D9811B8363D5FD5A` (break `/Game/Dati/Giocatore/MosseAttualiGiocatoreST` _skillgiocatore)))) :`NewEnumerator5` (`.Animazione_6_A2D9DE42406F882B081E8284B2054071` (break `/Game/Dati/Giocatore/MossaGiocatore` (`.AttaccoBase_35_7EA19321457B0FFDB2FA7F97ED10EF87` (break `/Game/Dati/Giocatore/MosseAttualiGiocatoreST` _skillgiocatore)))) :`NewEnumerator0` (`.Animazione_6_A2D9DE42406F882B081E8284B2054071` (break `/Game/Dati/Giocatore/MossaGiocatore` (`.SkillSlot1_23_FCAA49F04AA8105ED0B0FC959EB98725` (break `/Game/Dati/Giocatore/MosseAttualiGiocatoreST` _skillgiocatore)))) :`NewEnumerator1` (`.Animazione_6_A2D9DE42406F882B081E8284B2054071` (break `/Game/Dati/Giocatore/MossaGiocatore` (`.SkillSlot2_24_7C31ACA9462EC4BBFBD063AD9AE19358` (break `/Game/Dati/Giocatore/MosseAttualiGiocatoreST` _skillgiocatore)))) :`NewEnumerator2` (`.Animazione_6_A2D9DE42406F882B081E8284B2054071` (break `/Game/Dati/Giocatore/MossaGiocatore` (`.SkillSlot3_25_90B495E643884197A2E6CBB1100D88DA` (break `/Game/Dati/Giocatore/MosseAttualiGiocatoreST` _skillgiocatore)))))))
          (`/Game/Blueprint/BPAvversario.AggiornaVita` (`self.Nemico`) _returnvalue)
          (set `/Game/Blueprint/BPPersonaggio.MossaScelta` "NewEnumerator4" _giocatore_3)
          (bind (_direction_2 _newtrack_5_2) (`Timeline|Timeline_0` :!via `PlayFromStart`)
            (:`Update`
              (`self.MuoviInPosizione` _newtrack_5_2 (`self.PosAttaccoGiocatore`) (`self.PosGiocatore`) _giocatore_2))
            (:`Finished`
              (set `/Game/Blueprint/BPPersonaggio.InBattaglia` false _giocatore_2)
              (if (<= (`/Game/Blueprint/BPAvversario.Vita` _nemico_2) 0)
                (`self.NormalMode` true :!label _label)
                (else
                  (`self.Turno Avversario`))))))))
    (:`CastFailed`
      (cast `/Game/Blueprint/BPAvversario` ChiAttacca)
      (set `/Game/Blueprint/BPAvversario.InBattaglia` true _nemico)
      (set `/Game/Blueprint/BPAvversario.SkillNemicoEN` "NewEnumerator0" _nemico)
      (bind (_direction_3 _newtrack_5_3) (`Timeline|Timeline_2` :!via `PlayFromStart`)
        (:`Update`
          (`self.MuoviInPosizione` _newtrack_5_3 (`self.PosNemico`) (`self.PosAttaccoNemico`) _nemico_3))
        (:`Finished`
          (set `/Game/Blueprint/BPAvversario.SkillNemicoEN` "NewEnumerator2" _nemico_3)
          (`KismetSystemLibrary.Delay` (`PaperFlipbook.GetTotalDuration` _skillnemicost_skill1))
          (`/Game/Blueprint/BPPersonaggio.AggiornaVita` (`self.Giocatore`) _returnvalue)
          (set `/Game/Blueprint/BPAvversario.SkillNemicoEN` "NewEnumerator1" _nemico_3)
          (bind (_direction_4 _newtrack_5_4) (`Timeline|Timeline_3` :!via `PlayFromStart`)
            (:`Update`
              (`self.MuoviInPosizione` _newtrack_5_4 (`self.PosAttaccoNemico`) (`self.PosNemico`) _nemico_2))
            (:`Finished`
              (set `/Game/Blueprint/BPAvversario.InBattaglia` false _nemico_2)
              (if (<= (`/Game/Blueprint/BPPersonaggio.VIta` _giocatore_2) 0)
                (goto _label)
                (else
                  (bind _foundwidgets_2 (`WidgetBlueprintLibrary.GetAllWidgetsOfClass` "/Game/HUD/BPWidgetTurnoAvversario.BPWidgetTurnoAvversario_C"))
                  (for _array_element_2 _foundwidgets_2
                    (`Widget.RemoveFromParent` _array_element_2))
                  (`self.Turno Giocatore`))))))))))

(event `NormalMode`
  (params (Esito :type Boolean))
  (if Esito
    (`self.K2_DestroyActor` (`self.Nemico`))
    (bind _asbppersonaggio (cast `/Game/Blueprint/BPPersonaggio` (`GameplayStatics.GetPlayerCharacter` 0)))
    (`self.EnableInput` _asbppersonaggio null)
    (`/Game/Blueprint/BPPersonaggio.Carica Posizione` _asbppersonaggio)
    (`CharacterMovementComponent.SetMovementMode` (`Character.CharacterMovement` _asbppersonaggio) "MOVE_Flying" 0)
    (set `PlayerController.bShowMouseCursor` false (`GameplayStatics.GetPlayerController` 0))
    (`PlayerController.SetViewTargetWithBlend` (`GameplayStatics.GetPlayerController` 0) (`GameplayStatics.GetPlayerCharacter` 0) 0.0 "VTBlend_Linear" 0.0 false)
    (bind _asbphud (cast `/Game/HUD/BPHud` (`PlayerController.GetHUD` (`GameplayStatics.GetPlayerController` 0))))
    (`/Game/HUD/BPHud.HudNormale` _asbphud)
    (bind _outactors (`GameplayStatics.GetAllActorsOfClass` "/Game/Blueprint/BPAvversario.BPAvversario_C"))
    (for _array_element _outactors
      (`CharacterMovementComponent.SetMovementMode` (`Character.CharacterMovement` _array_element) "MOVE_Flying" 0)
      (set `/Game/Blueprint/BPAvversario.staInteragendo` false _array_element))))

(fn `MuoviInPosizione`
  (params (Lerp :type "Float (double-precision)") (PosizioneIniziale :type "Actor Object Reference") (PosizioneFinale :type "Actor Object Reference") (ChiDevoSpostare :type "PaperCharacter Object Reference"))
  (`self.K2_SetActorRelativeLocation` ChiDevoSpostare (`KismetMathLibrary.VLerp` (`self.K2_GetActorLocation` PosizioneIniziale) (`self.K2_GetActorLocation` PosizioneFinale) Lerp) false false))

(fn `UserConstructionScript`)