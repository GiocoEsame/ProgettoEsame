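; BPNPC is a merchant NPC that opens a market UI when interacted with.
; Interagisci creates a BPWIdgetMercato, passing OggettiInVendita as the merchant inventory, and adds it to the viewport.
; StopInteragisci hides the TextRender and removes every top-level market widget, found by class search rather than a stored reference.
; The node that shows the TextRender is unconnected, so this graph never makes it visible.
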(event `/Game/Blueprint/BPInterface.Interagisci`
  (bind _returnvalue (`|CreateWidget` "/Game/HUD/WidgetHUDGiocatore/BPWIdgetMercato.BPWIdgetMercato_C" null (`self.OggettiInVendita`)))
  (`UserWidget.AddToViewport` _returnvalue 0))

(event `/Game/Blueprint/BPInterface.StopInteragisci`
  (`SceneComponent.SetVisibility` (`self.TextRender`) false false)
  (bind _foundwidgets (`WidgetBlueprintLibrary.GetAllWidgetsOfClass` "/Game/HUD/WidgetHUDGiocatore/BPWIdgetMercato.BPWIdgetMercato_C"))
  (for _array_element _foundwidgets
    (`Widget.RemoveFromParent` _array_element)))

(fn `UserConstructionScript`)