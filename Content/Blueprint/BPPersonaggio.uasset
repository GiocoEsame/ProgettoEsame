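; Player character for a flipbook-sprite game, moving on X/Z with ladder use, health, coins and an inventory widget toggle.
; Each Tick, GestoreAnimazioni picks the flipbook from the battle move or last direction, also rotating the main collider outside battle.
; Overlapping a ladder with main and both side colliders snaps X and blocks horizontal input.
; Position and direction persist via BPSalvaGioco; items fill the first empty of eight struct slots.
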(event `InputAxis|MovimentoVerticale`
  (params (AxisValue :type "Float (single-precision)"))
  ;[1 1 1] Movimento
  (`self.AddMovementInput` (0.0 0.0 1.0) AxisValue))

(event `InputAxis|MovimentoOrizzontale`
  (params (AxisValue :type "Float (single-precision)"))
  ;[1 1 1] Movimento
  (if (not (`self.UtilizzaScala`))
    (`self.AddMovementInput` (1.0 0.0 0.0) AxisValue)))

(event `self.ReceiveTick`
  (params (DeltaSeconds :type "Float (single-precision)"))
  ;[1 1 1] Gestore animazioni
  (`self.GestoreAnimazioni`))

(event `self.ReceiveBeginPlay`
  (bind (_skillpossbiligiocatorest_posizioneattacco _skillpossbiligiocatorest_posizionenormale _skillpossbiligiocatorest_attaccobase _skillpossbiligiocatorest_skill1 _skillpossbiligiocatorest_skill2 _skillpossbiligiocatorest_skill3) (break `/Game/Dati/Giocatore/MossePossibiliGiocatoreST` (`self.SkillPossbiliGiocatoreST`)))
  (set `self.SkillGiocatore` (make `/Game/Dati/Giocatore/MosseAttualiGiocatoreST` _skillpossbiligiocatorest_posizioneattacco _skillpossbiligiocatorest_posizionenormale _skillpossbiligiocatorest_attaccobase _skillpossbiligiocatorest_skill1 _skillpossbiligiocatorest_skill2 _skillpossbiligiocatorest_skill3)))

(event `Carica Posizione`
  ;[1 1 1] Salvataggio e caricamento
  (bind _returnvalue (`GameplayStatics.DoesSaveGameExist` (`self.SaveSlot`)))
  (if _returnvalue
    (bind _returnvalue_2 (`GameplayStatics.LoadGameFromSlot` (`self.SaveSlot`)))
    (bind _output_get (set `self.SaverSubclass` _returnvalue_2))
    (bind _asbpsalva_gioco (cast `/Game/Blueprint/BPSalvaGioco` _output_get))
    (`self.K2_SetActorTransform` (`/Game/Blueprint/BPSalvaGioco.Posizione` _asbpsalva_gioco))
    (set `self.UltimaDirezione` (`/Game/Blueprint/BPSalvaGioco.Direzione` _asbpsalva_gioco))
    (else
      (bind _returnvalue_3 (`GameplayStatics.CreateSaveGameObject` "/Game/Blueprint/BPSalvaGioco.BPSalvaGioco_C" :!label _label))
      (bind _output_get_2 (set `self.SaverSubclass` _returnvalue_3))
      (bind _asbpsalva_gioco_2 (cast `/Game/Blueprint/BPSalvaGioco` _output_get_2))
      (set `/Game/Blueprint/BPSalvaGioco.Posizione` (`self.GetTransform`) _asbpsalva_gioco_2)
      (set `/Game/Blueprint/BPSalvaGioco.Direzione` (`self.UltimaDirezione`) _asbpsalva_gioco_2)
      (`GameplayStatics.SaveGameToSlot` (`self.SaverSubclass`) (`self.SaveSlot`))
      (`KismetSystemLibrary.PrintString` (`KismetStringLibrary.Conv_TransformToString` (`self.GetTransform`)) true true (struct :`R` 1.0 :`G` 0.035682 :`A` 1.0)))))

(event `Salva Posizione`
  ;[1 1 1] Salvataggio e caricamento
  (goto _label))

(event `self.CollisioneTotale.OnComponentBeginOverlap`
  (params (OverlappedComponent :type "PrimitiveComponent Object Reference") (OtherActor :type "Actor Object Reference") (OtherComp :type "PrimitiveComponent Object Reference") (OtherBodyIndex :type Integer) (bFromSweep :type Boolean) (SweepResult :type "HitResult Structure (by ref)"))
  (bind (_returnvalue_x _returnvalue_y _returnvalue_z) (`KismetMathLibrary.BreakVector` (`self.K2_GetActorLocation`)))
  ;[1 1 1] Utilizzo Scala
  (bind _asbpscala (cast `/Game/Blueprint/BPScala` OtherActor))
  (bind _output_get (set `self.VicinoScala` true))
  (if (and _output_get (and (stale `self.CollisioneFrontaleSX.OnComponentBeginOverlap` _output_get) (stale `self.CollisioneFrontaleDX.OnComponentBeginOverlap` _output_get))) :!label _label_2
    (set `self.UtilizzaScala` true)
    (bind _returnvalue_x_2 (`KismetMathLibrary.BreakVector` (`SceneComponent.K2_GetComponentLocation` (`/Game/Blueprint/BPScala.Box` _asbpscala))))
    (`self.K2_SetActorLocation` (`KismetMathLibrary.MakeVector` _returnvalue_x_2 _returnvalue_y _returnvalue_z))))

(event `self.CollisioneFrontaleSX.OnComponentBeginOverlap`
  (params (OverlappedComponent :type "PrimitiveComponent Object Reference") (OtherActor :type "Actor Object Reference") (OtherComp :type "PrimitiveComponent Object Reference") (OtherBodyIndex :type Integer) (bFromSweep :type Boolean) (SweepResult :type "HitResult Structure (by ref)"))
  ;[1 1 1] Utilizzo Scala
  (cast `/Game/Blueprint/BPScala` OtherActor
    (:`then`
      (bind _output_get (set `self.PuoInteragireSX` true))
      (goto _label_2))
    (:`CastFailed`
      (cast `/Game/Blueprint/BPNPC` (stale `self.CollisioneFrontaleDX.OnComponentBeginOverlap` OtherActor) :!label _label_3))))

(event `self.CollisioneFrontaleDX.OnComponentBeginOverlap`
  (params (OverlappedComponent :type "PrimitiveComponent Object Reference") (OtherActor :type "Actor Object Reference") (OtherComp :type "PrimitiveComponent Object Reference") (OtherBodyIndex :type Integer) (bFromSweep :type Boolean) (SweepResult :type "HitResult Structure (by ref)"))
  ;[1 1 1] Utilizzo Scala
  (cast `/Game/Blueprint/BPScala` OtherActor
    (:`then`
      (bind _output_get (set `self.PuoInteragireDX` true))
      (goto _label_2))
    (:`CastFailed`
      (goto _label_3))))

(event `self.CollisioneTotale.OnComponentEndOverlap`
  (params (OverlappedComponent :type "PrimitiveComponent Object Reference") (OtherActor :type "Actor Object Reference") (OtherComp :type "PrimitiveComponent Object Reference") (OtherBodyIndex :type Integer))
  ;[1 1 1] Utilizzo Scala
  (cast `/Game/Blueprint/BPScala` OtherActor)
  (set `self.PuoInteragireDX` false)
  (set `self.PuoInteragireSX` false)
  (set `self.VicinoScala` false)
  (set `self.UtilizzaScala` false))

(event `AggiornaVita`
  (params (Vita :type Integer))
  ;[1 1 1] Sistema della vita
  (set `self.VIta` (+ Vita (`self.VIta`))))

(event `InputAction|ApriInventario`
  (params (Key :type "Key Structure"))
  (:`Pressed`
    (`/Engine/EditorBlueprintResources/StandardMacros.FlipFlop`
      (:`A`
        (bind _returnvalue (`|CreateWidget` "/Game/HUD/BPWidgetInventario.BPWidgetInventario_C"))
        (bind _output_get (set `self.WidgetInventario` _returnvalue))
        (`UserWidget.AddToViewport` _output_get 0)
        (set `PlayerController.bShowMouseCursor` true (`GameplayStatics.GetPlayerController` 0))
        (`WidgetBlueprintLibrary.SetInputMode_GameAndUIEx` (`GameplayStatics.GetPlayerController` 0) _output_get))
      (:`B`
        (`Widget.RemoveFromParent` (`self.WidgetInventario`))))))

(event `AggiornaMonete`
  (params (Monete :type Integer))
  (set `self.Monete` (+ Monete (`self.Monete`))))

(event `ModificaSlotInventario`
  (params (idOggetto :type "/Game/Dati/OggettoST Structure"))
  (bind _inventario (`self.Inventario`))
  (bind _oggettoinserito (`self.InserisciInInventario` idOggetto))
  (`KismetSystemLibrary.PrintString` (`KismetStringLibrary.Conv_BoolToString` _oggettoinserito))
  (`KismetSystemLibrary.PrintString` (`KismetStringLibrary.Concat_StrStr` (`KismetStringLibrary.Conv_IntToString` (break `/Game/Dati/OggettoST` (break `/Game/Dati/Giocatore/InventarioST` _inventario))) (`KismetStringLibrary.Conv_IntToString` (break `/Game/Dati/OggettoST` (`.InvSlot2_51_82CC520842AA12A411CEF98688687AD4` (break `/Game/Dati/Giocatore/InventarioST` _inventario)))) (`KismetStringLibrary.Conv_IntToString` (break `/Game/Dati/OggettoST` (`.InvSlot3_44_5F3ACE9443A76B5220676AB0AE0FFEDF` (break `/Game/Dati/Giocatore/InventarioST` _inventario)))) (`KismetStringLibrary.Conv_IntToString` (break `/Game/Dati/OggettoST` (`.InvSlot4_45_20D6AC274FEAF8A85D678E9C6227D3E1` (break `/Game/Dati/Giocatore/InventarioST` _inventario)))) (`KismetStringLibrary.Conv_IntToString` (break `/Game/Dati/OggettoST` (`.InvSlot5_46_ACD898FF4ACDDA233EF77A98D68DF8FC` (break `/Game/Dati/Giocatore/InventarioST` _inventario)))) (`KismetStringLibrary.Conv_IntToString` (break `/Game/Dati/OggettoST` (`.InvSlot6_47_C07466E848BDE43A9C8A5CBCB2006ADA` (break `/Game/Dati/Giocatore/InventarioST` _inventario)))) (`KismetStringLibrary.Conv_IntToString` (break `/Game/Dati/OggettoST` (`.InvSlot7_48_9E7646864ECF514688FBE3A23CF821A6` (break `/Game/Dati/Giocatore/InventarioST` _inventario)))) (`KismetStringLibrary.Conv_IntToString` (break `/Game/Dati/OggettoST` (`.InvSlot8_49_C3EAAEF84336925C8E7DB1B0905F6775` (break `/Game/Dati/Giocatore/InventarioST` _inventario))))) true true (struct :`R` 1.0 :`G` 0.153517 :`A` 1.0)))

(fn `GestoreAnimazioni`
  (bind _returnvalue (`self.GetInputAxisValue`))
  (bind _returnvalue_2 (`self.GetInputAxisValue`))
  (bind (_animazionipersonaggio_muovisu _animazionipersonaggio_idlesu _animazionipersonaggio_muovigiu _animazionipersonaggio_idlegiu _animazionipersonaggio_muovisinistra _animazionipersonaggio_idlesinistra _animazionipersonaggio_muovidestra _animazionipersonaggio_idledestra _animazionipersonaggio_scalasu _animazionipersonaggio_scalagiu) (break `/Game/Dati/Giocatore/MovimentoGiocatoreST` (`self.AnimazioniPersonaggio`)))
  (bind _utilizzascala (`self.UtilizzaScala`))
  (bind _ultimadirezione (`self.UltimaDirezione`))
  (bind (_skillgiocatore_posizioneattacco _skillgiocatore_posizionedifesa _skillgiocatore_attaccobase _skillgiocatore_skillslot1 _skillgiocatore_skillslot2 _skillgiocatore_skillslot3) (break `/Game/Dati/Giocatore/MosseAttualiGiocatoreST` (`self.SkillGiocatore`)))
  (bind _skillpossbiligiocatorest (`self.SkillPossbiliGiocatoreST`))
  (bind _returnvalue_3 (< _returnvalue_2 0.0))
  (bind _returnvalue_4 (not (`self.UtilizzaScala`)))
  (bind _returnvalue_5 (> _returnvalue_2 0.0))
  (bind _returnvalue_idmossa (break `/Game/Dati/Giocatore/MossaGiocatore` (select `/Game/Dati/Giocatore/MosseGiocatoreEN` (`self.MossaScelta`) :`NewEnumerator3` _skillgiocatore_posizioneattacco :`NewEnumerator4` _skillgiocatore_posizionedifesa :`NewEnumerator5` _skillgiocatore_attaccobase :`NewEnumerator0` _skillgiocatore_skillslot1 :`NewEnumerator1` _skillgiocatore_skillslot2 :`NewEnumerator2` _skillgiocatore_skillslot3)))
  (if (`self.InBattaglia`)
    (`PaperFlipbookComponent.SetFlipbook` (`self.Sprite`) (select `int` _returnvalue_idmossa :`0` (`.Animazione_6_A2D9DE42406F882B081E8284B2054071` (break `/Game/Dati/Giocatore/MossaGiocatore` (break `/Game/Dati/Giocatore/MossePossibiliGiocatoreST` _skillpossbiligiocatorest))) :`1` (`.Animazione_6_A2D9DE42406F882B081E8284B2054071` (break `/Game/Dati/Giocatore/MossaGiocatore` (`.PosizioneNormale_18_A8EC926747EBBE8681EE14AD2E6D8939` (break `/Game/Dati/Giocatore/MossePossibiliGiocatoreST` _skillpossbiligiocatorest)))) :`2` (`.Animazione_6_A2D9DE42406F882B081E8284B2054071` (break `/Game/Dati/Giocatore/MossaGiocatore` (`.AttaccoBase_19_AB00896740E39F52C9643E870581EF13` (break `/Game/Dati/Giocatore/MossePossibiliGiocatoreST` _skillpossbiligiocatorest)))) :`3` (`.Animazione_6_A2D9DE42406F882B081E8284B2054071` (break `/Game/Dati/Giocatore/MossaGiocatore` (`.Skill1_20_68BC577444EB4BE753052A94ED547BC0` (break `/Game/Dati/Giocatore/MossePossibiliGiocatoreST` _skillpossbiligiocatorest)))) :`4` (`.Animazione_6_A2D9DE42406F882B081E8284B2054071` (break `/Game/Dati/Giocatore/MossaGiocatore` (`.Skill2_22_E38DEE3D448D65FA18AC16AC8E9AE1D2` (break `/Game/Dati/Giocatore/MossePossibiliGiocatoreST` _skillpossbiligiocatorest)))) :`5` (`.Animazione_6_A2D9DE42406F882B081E8284B2054071` (break `/Game/Dati/Giocatore/MossaGiocatore` (`.Skill2_22_E38DEE3D448D65FA18AC16AC8E9AE1D2` (break `/Game/Dati/Giocatore/MossePossibiliGiocatoreST` _skillpossbiligiocatorest))))))
    (else
      (if (or (!= (`self.GetInputAxisValue`) 0.0) (!= (`self.GetInputAxisValue`) 0.0))
        (if (and _utilizzascala _returnvalue_5)
          (set `self.UltimaDirezione` "NewEnumerator4")
          (elif (and _utilizzascala _returnvalue_3)
            (set `self.UltimaDirezione` "NewEnumerator5")
            (elif _returnvalue_5
              (set `self.UltimaDirezione` "NewEnumerator0")
              (elif _returnvalue_3
                (set `self.UltimaDirezione` "NewEnumerator1")
                (elif (and _returnvalue_4 (> _returnvalue 0.0))
                  (set `self.UltimaDirezione` "NewEnumerator3")
                  (elif (and _returnvalue_4 (< _returnvalue 0.0))
                    (set `self.UltimaDirezione` "NewEnumerator2"))))))))
      (`SceneComponent.K2_SetRelativeRotation` (`self.CollisioneTotale`) (select `/Game/Dati/Giocatore/MovimentoGiocatoreEN` (`self.UltimaDirezione`) :`NewEnumerator1` (struct :`Pitch` 180.0) :`NewEnumerator2` (struct :`Pitch` 90.0) :`NewEnumerator3` (struct :`Pitch` 270.0) :`NewEnumerator5` (struct :`Pitch` 180.0) :!type "Rotator Structure") false false)
      (`PaperFlipbookComponent.SetFlipbook` (`self.Sprite`) (select `bool` (> (`KismetMathLibrary.VSize` (`self.GetVelocity`)) 0.0) :`false` (select `/Game/Dati/Giocatore/MovimentoGiocatoreEN` _ultimadirezione :`NewEnumerator0` _animazionipersonaggio_idlesu :`NewEnumerator1` _animazionipersonaggio_idlegiu :`NewEnumerator2` _animazionipersonaggio_idlesinistra :`NewEnumerator3` _animazionipersonaggio_idledestra :`NewEnumerator4` _animazionipersonaggio_scalasu :`NewEnumerator5` _animazionipersonaggio_scalagiu) :`true` (select `/Game/Dati/Giocatore/MovimentoGiocatoreEN` _ultimadirezione :`NewEnumerator0` _animazionipersonaggio_muovisu :`NewEnumerator1` _animazionipersonaggio_muovigiu :`NewEnumerator2` _animazionipersonaggio_muovisinistra :`NewEnumerator3` _animazionipersonaggio_muovidestra :`NewEnumerator4` _animazionipersonaggio_scalasu :`NewEnumerator5` _animazionipersonaggio_scalagiu))))))

(fn `InserisciInInventario`
  (params (idOggetto :type "/Game/Dati/OggettoST Structure"))
  (returns (OggettoInserito :type Boolean))
  (locals (slotInventario :type Integer))
  (bind _inventario (`self.Inventario`))
  (if (== (break `/Game/Dati/OggettoST` (break `/Game/Dati/Giocatore/InventarioST` _inventario)) 0)
    (set `local.slotInventario` 1)
    (elif (== (break `/Game/Dati/OggettoST` (`.InvSlot2_51_82CC520842AA12A411CEF98688687AD4` (break `/Game/Dati/Giocatore/InventarioST` _inventario))) 0)
      (set `local.slotInventario` 2)
      (elif (== (break `/Game/Dati/OggettoST` (`.InvSlot3_44_5F3ACE9443A76B5220676AB0AE0FFEDF` (break `/Game/Dati/Giocatore/InventarioST` _inventario))) 0)
        (set `local.slotInventario` 3)
        (elif (== (break `/Game/Dati/OggettoST` (`.InvSlot4_45_20D6AC274FEAF8A85D678E9C6227D3E1` (break `/Game/Dati/Giocatore/InventarioST` _inventario))) 0)
          (set `local.slotInventario` 4)
          (elif (== (break `/Game/Dati/OggettoST` (`.InvSlot5_46_ACD898FF4ACDDA233EF77A98D68DF8FC` (break `/Game/Dati/Giocatore/InventarioST` _inventario))) 0)
            (set `local.slotInventario` 5)
            (elif (== (break `/Game/Dati/OggettoST` (`.InvSlot6_47_C07466E848BDE43A9C8A5CBCB2006ADA` (break `/Game/Dati/Giocatore/InventarioST` _inventario))) 0)
              (set `local.slotInventario` 6)
              (elif (== (break `/Game/Dati/OggettoST` (`.InvSlot7_48_9E7646864ECF514688FBE3A23CF821A6` (break `/Game/Dati/Giocatore/InventarioST` _inventario))) 0)
                (set `local.slotInventario` 7)
                (elif (== (break `/Game/Dati/OggettoST` (`.InvSlot8_49_C3EAAEF84336925C8E7DB1B0905F6775` (break `/Game/Dati/Giocatore/InventarioST` _inventario))) 0)
                  (set `local.slotInventario` 8)
                  (else
                    (return false))))))))))
  (`self.ModificaInventario` (`local.slotInventario`) idOggetto)
  (return true))

(fn `ModificaInventario`
  (params (NumeroSlot :type Integer) (Oggetto :type "/Game/Dati/OggettoST Structure"))
  (bind (_inventario_invslot1 _inventario_invslot2 _inventario_invslot3 _inventario_invslot4 _inventario_invslot5 _inventario_invslot6 _inventario_invslot7 _inventario_invslot8) (break `/Game/Dati/Giocatore/InventarioST` (`self.Inventario`)))
  (if (== NumeroSlot 1)
    (set `self.Inventario` (make `/Game/Dati/Giocatore/InventarioST` Oggetto _inventario_invslot2 _inventario_invslot3 _inventario_invslot4 _inventario_invslot5 _inventario_invslot6 _inventario_invslot7 _inventario_invslot8))
    (elif (== NumeroSlot 2)
      (set `self.Inventario` (make `/Game/Dati/Giocatore/InventarioST` _inventario_invslot1 Oggetto _inventario_invslot3 _inventario_invslot4 _inventario_invslot5 _inventario_invslot6 _inventario_invslot7 _inventario_invslot8))
      (elif (== NumeroSlot 3)
        (set `self.Inventario` (make `/Game/Dati/Giocatore/InventarioST` _inventario_invslot1 _inventario_invslot2 Oggetto _inventario_invslot4 _inventario_invslot5 _inventario_invslot6 _inventario_invslot7 _inventario_invslot8))
        (elif (== NumeroSlot 4)
          (set `self.Inventario` (make `/Game/Dati/Giocatore/InventarioST` _inventario_invslot1 _inventario_invslot2 _inventario_invslot3 Oggetto _inventario_invslot5 _inventario_invslot6 _inventario_invslot7 _inventario_invslot8))
          (elif (== NumeroSlot 5)
            (set `self.Inventario` (make `/Game/Dati/Giocatore/InventarioST` _inventario_invslot1 _inventario_invslot2 _inventario_invslot3 _inventario_invslot4 Oggetto _inventario_invslot6 _inventario_invslot7 _inventario_invslot8))
            (elif (== NumeroSlot 6)
              (set `self.Inventario` (make `/Game/Dati/Giocatore/InventarioST` _inventario_invslot1 _inventario_invslot2 _inventario_invslot3 _inventario_invslot4 _inventario_invslot5 Oggetto _inventario_invslot7 _inventario_invslot8))
              (elif (== NumeroSlot 7)
                (set `self.Inventario` (make `/Game/Dati/Giocatore/InventarioST` _inventario_invslot1 _inventario_invslot2 _inventario_invslot3 _inventario_invslot4 _inventario_invslot5 _inventario_invslot6 Oggetto _inventario_invslot8))
                (elif (== NumeroSlot 8)
                  (set `self.Inventario` (make `/Game/Dati/Giocatore/InventarioST` _inventario_invslot1 _inventario_invslot2 _inventario_invslot3 _inventario_invslot4 _inventario_invslot5 _inventario_invslot6 _inventario_invslot7 Oggetto)))))))))))

(fn `UserConstructionScript`)