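; Base Paper2D player character that moves on the X/Z plane, climbs BPScala ladders and saves or loads its state.
; Tick derives the last direction from input, rotating the interaction box and choosing walk, idle or ladder flipbooks.
; Box plus both front colliders overlapping a ladder snaps X to it and blocks horizontal movement.
; Debug keys save, load and print the transform via BPSalvaGioco; StartBattle is an empty stub.
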(event `InputAxis|MovimentoVerticale`
  (params (AxisValue :type "Float (single-precision)"))
  ;[1 1 1] Movimento
  (`self.AddMovementInput` (0.0 0.0 1.0) AxisValue))

(event `InputAxis|MovimentoOrizzontale`
  (params (AxisValue :type "Float (single-precision)"))
  ;[1 1 1] Movimento
  (if (not (`self.UtilizzaScala`))
    (`self.AddMovementInput` (1.0 0.0 0.0) AxisValue)))

(event `self.ReceiveTick`
  (params (DeltaSeconds :type "Float (single-precision)"))
  ;[1 1 1] Gestore animazioni
  (`self.GestoreAnimazioni`))

(event `Key|K`
  (params (Key :type "Key Structure"))
  ;[1 1 1] Salvataggio e caricamento
  (:`Pressed`
    (bind _returnvalue (`GameplayStatics.DoesSaveGameExist` (`self.SaveSlot`)))
    (if _returnvalue
      (bind _returnvalue_2 (`GameplayStatics.LoadGameFromSlot` (`self.SaveSlot`)))
      (bind _output_get (set `self.SaverSubclass` _returnvalue_2))
      (bind _asbpsalva_gioco (cast `/Game/Blueprint/BPSalvaGioco` _output_get))
      (`self.K2_SetActorTransform` (`/Game/Blueprint/BPSalvaGioco.Posizione` _asbpsalva_gioco))
      (set `self.UltimaDirezione` (`/Game/Blueprint/BPSalvaGioco.Direzione` _asbpsalva_gioco))
      (else
        (bind _returnvalue_3 (`GameplayStatics.CreateSaveGameObject` "/Game/Blueprint/BPSalvaGioco.BPSalvaGioco_C" :!label _label))
        (bind _output_get_2 (set `self.SaverSubclass` _returnvalue_3))
        (bind _asbpsalva_gioco_2 (cast `/Game/Blueprint/BPSalvaGioco` _output_get_2))
        (set `/Game/Blueprint/BPSalvaGioco.Posizione` (`self.GetTransform`) _asbpsalva_gioco_2)
        (set `/Game/Blueprint/BPSalvaGioco.Direzione` (`self.UltimaDirezione`) _asbpsalva_gioco_2)
        (`GameplayStatics.SaveGameToSlot` (`self.SaverSubclass`) (`self.SaveSlot`))
        (`KismetSystemLibrary.PrintString` (`KismetStringLibrary.Conv_TransformToString` (`self.GetTransform`)) true true (struct :`R` 1.0 :`G` 0.035682 :`A` 1.0))))))

(event `Key|J`
  (params (Key :type "Key Structure"))
  ;[1 1 1] Salvataggio e caricamento
  (:`Pressed`
    (goto _label)))

(event `Key|H`
  (params (Key :type "Key Structure"))
  ;[1 1 1] Debug
  (:`Pressed`
    (`KismetSystemLibrary.PrintString` (`KismetStringLibrary.Conv_TransformToString` (`self.GetTransform`)))))

(event `self.Box.OnComponentBeginOverlap`
  (params (OverlappedComponent :type "PrimitiveComponent Object Reference") (OtherActor :type "Actor Object Reference") (OtherComp :type "PrimitiveComponent Object Reference") (OtherBodyIndex :type Integer) (bFromSweep :type Boolean) (SweepResult :type "HitResult Structure (by ref)"))
  (bind (_returnvalue_x _returnvalue_y _returnvalue_z) (`KismetMathLibrary.BreakVector` (`self.K2_GetActorLocation`)))
  (bind _asbpscala (cast `/Game/Blueprint/BPScala` OtherActor))
  (bind _output_get (set `self.VicinoScala` true))
  (if (and _output_get (and (stale `self.ColisioneFrontaleSX.OnComponentBeginOverlap` _output_get) (stale `self.CollisioneFrontaleDX.OnComponentBeginOverlap` _output_get))) :!label _label_2
    (set `self.UtilizzaScala` true)
    (bind _returnvalue_x_2 (`KismetMathLibrary.BreakVector` (`SceneComponent.K2_GetComponentLocation` (`/Game/Blueprint/BPScala.Box` _asbpscala))))
    (`self.K2_SetActorLocation` (`KismetMathLibrary.MakeVector` _returnvalue_x_2 _returnvalue_y _returnvalue_z))))

(event `self.ColisioneFrontaleSX.OnComponentBeginOverlap`
  (params (OverlappedComponent :type "PrimitiveComponent Object Reference") (OtherActor :type "Actor Object Reference") (OtherComp :type "PrimitiveComponent Object Reference") (OtherBodyIndex :type Integer) (bFromSweep :type Boolean) (SweepResult :type "HitResult Structure (by ref)"))
  (cast `/Game/Blueprint/BPScala` OtherActor)
  (bind _output_get (set `self.PuoInteragireSX` true))
  (goto _label_2))

(event `self.CollisioneFrontaleDX.OnComponentBeginOverlap`
  (params (OverlappedComponent :type "PrimitiveComponent Object Reference") (OtherActor :type "Actor Object Reference") (OtherComp :type "PrimitiveComponent Object Reference") (OtherBodyIndex :type Integer) (bFromSweep :type Boolean) (SweepResult :type "HitResult Structure (by ref)"))
  (cast `/Game/Blueprint/BPScala` OtherActor)
  (bind _output_get (set `self.PuoInteragireDX` true))
  (goto _label_2))

(event `self.Box.OnComponentEndOverlap`
  (params (OverlappedComponent :type "PrimitiveComponent Object Reference") (OtherActor :type "Actor Object Reference") (OtherComp :type "PrimitiveComponent Object Reference") (OtherBodyIndex :type Integer))
  (cast `/Game/Blueprint/BPScala` OtherActor)
  (set `self.PuoInteragireDX` false)
  (set `self.PuoInteragireSX` false)
  (set `self.VicinoScala` false)
  (set `self.UtilizzaScala` false))

(fn `GestoreAnimazioni`
  (bind _returnvalue (`self.GetInputAxisValue`))
  (bind _returnvalue_2 (`self.GetInputAxisValue`))
  (bind (_animazionipersonaggio_muovisu _animazionipersonaggio_idlesu _animazionipersonaggio_muovigiu _animazionipersonaggio_idlegiu _animazionipersonaggio_muovisinistra _animazionipersonaggio_idlesinistra _animazionipersonaggio_muovidestra _animazionipersonaggio_idledestra _animazionipersonaggio_scalasu _animazionipersonaggio_scalagiu) (break `/Game/Dati/MovimentoGiocatoreST` (`self.AnimazioniPersonaggio`)))
  (bind _utilizzascala (`self.UtilizzaScala`))
  (bind _ultimadirezione (`self.UltimaDirezione`))
  (bind _returnvalue_3 (< _returnvalue_2 0.0))
  (bind _returnvalue_4 (not (`self.UtilizzaScala`)))
  (bind _returnvalue_5 (> _returnvalue_2 0.0))
  (if (or (!= (`self.GetInputAxisValue`) 0.0) (!= (`self.GetInputAxisValue`) 0.0))
    (if (and _utilizzascala _returnvalue_5)
      (set `self.UltimaDirezione` "NewEnumerator4")
      (elif (and _utilizzascala _returnvalue_3)
        (set `self.UltimaDirezione` "NewEnumerator5")
        (elif _returnvalue_5
          (set `self.UltimaDirezione` "NewEnumerator0")
          (elif _returnvalue_3
            (set `self.UltimaDirezione` "NewEnumerator1")
            (elif (and _returnvalue_4 (> _returnvalue 0.0))
              (set `self.UltimaDirezione` "NewEnumerator3")
              (elif (and _returnvalue_4 (< _returnvalue 0.0))
                (set `self.UltimaDirezione` "NewEnumerator2"))))))))
  (`SceneComponent.K2_SetRelativeRotation` (`self.Box`) (select `/Game/Dati/MovimentoGiocatoreEN` (`self.UltimaDirezione`) :`NewEnumerator1` (struct :`Pitch` 180.0) :`NewEnumerator2` (struct :`Pitch` 90.0) :`NewEnumerator3` (struct :`Pitch` 270.0) :`NewEnumerator5` (struct :`Pitch` 180.0) :!type "Rotator Structure") false false)
  (`PaperFlipbookComponent.SetFlipbook` (`self.Sprite`) (select `bool` (> (`KismetMathLibrary.VSize` (`self.GetVelocity`)) 0.0) :`false` (select `/Game/Dati/MovimentoGiocatoreEN` _ultimadirezione :`NewEnumerator0` _animazionipersonaggio_idlesu :`NewEnumerator1` _animazionipersonaggio_idlegiu :`NewEnumerator2` _animazionipersonaggio_idlesinistra :`NewEnumerator3` _animazionipersonaggio_idledestra :`NewEnumerator4` _animazionipersonaggio_scalasu :`NewEnumerator5` _animazionipersonaggio_scalagiu) :`true` (select `/Game/Dati/MovimentoGiocatoreEN` _ultimadirezione :`NewEnumerator0` _animazionipersonaggio_muovisu :`NewEnumerator1` _animazionipersonaggio_muovigiu :`NewEnumerator2` _animazionipersonaggio_muovisinistra :`NewEnumerator3` _animazionipersonaggio_muovidestra :`NewEnumerator4` _animazionipersonaggio_scalasu :`NewEnumerator5` _animazionipersonaggio_scalagiu)))
  (if (`KismetSystemLibrary.IsValid` (`self.CollisioneFrontaleDX`))
    _))

(fn `StartBattle`
  (params (Nemico :type Boolean) (Scenario :type "/Game/Dati/ScenariEN Enum" :default "ScenariEN_MAX")))

(fn `UserConstructionScript`)