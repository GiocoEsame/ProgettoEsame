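; Quest-capable NPC with a name label, dialogue and an optional Quest class to give the player.
; AttivaTesto and DisattivaTesto swap the label's material and "[F]" prompt for quest NPCs, but only toggle name visibility for others.
; Interagisci passes itself, name and dialogue to the player HUD and animates the text in; StopInteragisci reverses it.
; AssegnaQuest adds and starts the quest through the player's QuestManager unless already listed.
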(event `/Game/Blueprint/BPInterface.AttivaTesto`
  (bind _testo (`self.Testo`))
  (if (`KismetSystemLibrary.IsValidClass` (`self.Quest`))
    (`PrimitiveComponent.SetMaterial` _testo 0 "/Game/Grafica/MaterialeNPCNormale.MaterialeNPCNormale")
    (`TextRenderComponent.K2_SetText` (`self.Testo`) (`KismetTextLibrary.Conv_StringToText` (`KismetStringLibrary.Concat_StrStr` (`self.Nome`) " [F]")))
    (else
      (`SceneComponent.SetVisibility` _testo true false))))

(event `/Game/Blueprint/BPInterface.DisattivaTesto`
  (bind _testo (`self.Testo`))
  (if (`KismetSystemLibrary.IsValidClass` (`self.Quest`)) :!label _label
    (`PrimitiveComponent.SetMaterial` _testo 0 "/Game/Grafica/MaterialeNPCQuest.MaterialeNPCQuest")
    (`TextRenderComponent.K2_SetText` (`self.Testo`) (`KismetTextLibrary.Conv_StringToText` (`self.Nome`)))
    (else
      (`SceneComponent.SetVisibility` _testo false false))))

(event `self.ReceiveBeginPlay`
  (`TextRenderComponent.K2_SetText` (`self.Testo`) (`KismetTextLibrary.Conv_StringToText` (`self.Nome`)))
  (goto _label))

(event `/Game/Blueprint/BPInterface.Interagisci`
  (params (Personaggio :type "/Game/Blueprint/BPPersonaggio Object Reference"))
  (bind _hudgiocatore (`/Game/Blueprint/BPPersonaggio.HUDGiocatore` Personaggio))
  (set `/Game/HUD/WidgetHUDGiocatore/BPWIdgetHudGiocatore.Actor` self _hudgiocatore)
  (set `/Game/HUD/WidgetHUDGiocatore/BPWIdgetHudGiocatore.Nome` (`self.Nome`) _hudgiocatore)
  (set `/Game/HUD/WidgetHUDGiocatore/BPWIdgetHudGiocatore.Testo` (`self.Dialogo`) _hudgiocatore)
  (`UserWidget.PlayAnimation` _hudgiocatore (`/Game/HUD/WidgetHUDGiocatore/BPWIdgetHudGiocatore.AppareTesto` _hudgiocatore) 0.0 1 "Forward" 1.0))

(event `/Game/Blueprint/BPInterface.StopInteragisci`
  (bind _hudgiocatore (`/Game/Blueprint/BPPersonaggio.HUDGiocatore` (cast `/Game/Blueprint/BPPersonaggio` (`GameplayStatics.GetPlayerCharacter` 0) :!pure true)))
  (set `self.Aperto` false)
  (`UserWidget.PlayAnimation` _hudgiocatore (`/Game/HUD/WidgetHUDGiocatore/BPWIdgetHudGiocatore.AppareTesto` _hudgiocatore) 0.0 1 "Reverse" 1.0))

(event `AssegnaQuest`
  (bind _quest (`self.Quest`))
  (bind _questmanager (`/Game/Blueprint/BPPersonaggio.QuestManager` (cast `/Game/Blueprint/BPPersonaggio` (`GameplayStatics.GetPlayerCharacter` 0) :!pure true)))
  (if (not (`KismetArrayLibrary.Array_Contains` (`/Game/Dati/SistemaQuest/Actors/BpQuestManager.TutteLeQuest` _questmanager) _quest))
    (`/Game/Dati/SistemaQuest/Actors/BpQuestManager.AggiungiQuest` _questmanager _quest true)))

(fn `UserConstructionScript`)