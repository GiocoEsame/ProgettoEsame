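; BPCartello is an interactable sign (cartello) that shows its name and text in the player's HUD.
; The first Interagisci call registers the sign with the HUD, resets the text index, fills in the text and plays the appear animation; later calls advance the text through ContinuaTesto.
; DisattivaTesto plays that animation in reverse on player 0's HUD and clears the Aperto open flag.
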(event `/Game/Blueprint/BPInterface.Interagisci`
  (params (Personaggio :type "/Game/Blueprint/BPPersonaggio Object Reference"))
  (bind _hudgiocatore (`/Game/Blueprint/BPPersonaggio.HUDGiocatore` Personaggio))
  (if (`self.Aperto`)
    (`/Game/HUD/WidgetHUDGiocatore/BPWIdgetHudGiocatore.ContinuaTesto` _hudgiocatore)
    (else
      (set `/Game/HUD/WidgetHUDGiocatore/BPWIdgetHudGiocatore.IndiceTesto` 0 _hudgiocatore)
      (set `/Game/HUD/WidgetHUDGiocatore/BPWIdgetHudGiocatore.NPC` self _hudgiocatore)
      (if true
        (set `/Game/HUD/WidgetHUDGiocatore/BPWIdgetHudGiocatore.Nome` (`self.Nome`) _hudgiocatore)
        (set `/Game/HUD/WidgetHUDGiocatore/BPWIdgetHudGiocatore.Testo` (`self.TestoChiave`) _hudgiocatore)
        (`UserWidget.PlayAnimation` _hudgiocatore (`/Game/HUD/WidgetHUDGiocatore/BPWIdgetHudGiocatore.AppareTesto` _hudgiocatore) 0.0 1 "Forward" 1.0)
        (set `self.Aperto` true)))))

(event `/Game/Blueprint/BPInterface.DisattivaTesto`
  (bind _hudgiocatore (`/Game/Blueprint/BPPersonaggio.HUDGiocatore` (cast `/Game/Blueprint/BPPersonaggio` (`GameplayStatics.GetPlayerCharacter` 0) :!pure true)))
  (if (`self.Aperto`)
    (`UserWidget.PlayAnimation` _hudgiocatore (`/Game/HUD/WidgetHUDGiocatore/BPWIdgetHudGiocatore.AppareTesto` _hudgiocatore) 0.0 1 "Reverse" 1.0)
    (set `self.Aperto` false)))

(fn `UserConstructionScript`)