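; Key actor that opens its linked door when the player character overlaps it, or shows dialogue when it has text.
; Without text, overlap opens Porta, destroys the Oscuramenti actors and itself, and plays the key-found sound through GestoreSuoni.
; With text, overlap does nothing; Interagisci shows or advances the text on the player HUD and DisattivaTesto reverses its animation.
; The construction script applies the chosen Paper2D sprite.
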(event `self.ReceiveBeginPlay`
  (set `self.HaTesto?` (> (`KismetArrayLibrary.Array_Length` (`self.TestoChiave`)) 0)))

(event `self.ReceiveActorBeginOverlap`
  (params (OtherActor :type "Actor Object Reference"))
  (if (not (`self.HaTesto?`))
    (cast `/Game/Blueprint/BPPersonaggio` OtherActor)
    (`/Game/Blueprint/PortaEChiave/BPPorta1.ApriPorta` (`self.Porta`))
    (for _array_element (`self.Oscuramenti`)
      (`/Engine/EditorBlueprintResources/StandardMacros.IsValid` _array_element
        (:`Is Valid`
          (`self.K2_DestroyActor` _array_element))))
    (`self.K2_DestroyActor`)
    (bind _outactors (`GameplayStatics.GetAllActorsOfClass` "/Game/Blueprint/GestoreSuoni.GestoreSuoni_C"))
    (for _array_element_2 _outactors
      (`/Game/Blueprint/GestoreSuoni.PlayEffect` _array_element_2 "/Game/MusicaEsuoni/ChiaveTrovata.ChiaveTrovata"))))

(event `/Game/Blueprint/BPInterface.Interagisci`
  (params (Personaggio :type "/Game/Blueprint/BPPersonaggio Object Reference"))
  (bind _hudgiocatore (`/Game/Blueprint/BPPersonaggio.HUDGiocatore` Personaggio))
  (if (`self.Aperto`)
    (`/Game/HUD/WidgetHUDGiocatore/BPWIdgetHudGiocatore.ContinuaTesto` _hudgiocatore)
    (else
      (set `/Game/HUD/WidgetHUDGiocatore/BPWIdgetHudGiocatore.IndiceTesto` 0 _hudgiocatore)
      (set `/Game/HUD/WidgetHUDGiocatore/BPWIdgetHudGiocatore.NPC` self _hudgiocatore)
      (if true
        (set `/Game/HUD/WidgetHUDGiocatore/BPWIdgetHudGiocatore.Nome` (`self.Nome`) _hudgiocatore)
        (set `/Game/HUD/WidgetHUDGiocatore/BPWIdgetHudGiocatore.Testo` (`self.TestoChiave`) _hudgiocatore)
        (`UserWidget.PlayAnimation` _hudgiocatore (`/Game/HUD/WidgetHUDGiocatore/BPWIdgetHudGiocatore.AppareTesto` _hudgiocatore) 0.0 1 "Forward" 1.0)
        (set `self.Aperto` true)))))

(event `/Game/Blueprint/BPInterface.DisattivaTesto`
  (bind _hudgiocatore (`/Game/Blueprint/BPPersonaggio.HUDGiocatore` (cast `/Game/Blueprint/BPPersonaggio` (`GameplayStatics.GetPlayerCharacter` 0) :!pure true)))
  (if (`self.HaTesto?`)
    (`UserWidget.PlayAnimation` _hudgiocatore (`/Game/HUD/WidgetHUDGiocatore/BPWIdgetHudGiocatore.AppareTesto` _hudgiocatore) 0.0 1 "Reverse" 1.0)
    (set `self.Aperto` false)))

(fn `UserConstructionScript`
  (`PaperSpriteComponent.SetSprite` (`self.PaperSprite`) (`self.Sprite`)))