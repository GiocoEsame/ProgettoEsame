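; BPCassa is an interactable loot chest that opens and closes a UI showing its Drop contents.
; Interagisci toggles the Aperto flag, either creating a BPWIdgetCassa fed with Drop and a self reference or closing it; StopInteragisci always closes.
; Closing removes all top-level chest widgets and, for each, selected-object widgets whose Provenienza matches one enum value.
; AttivaTesto and DisattivaTesto toggle the Testo prompt, hidden at BeginPlay.
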(event `/Game/Blueprint/BPInterface.Interagisci`
  (if (`self.Aperto`)
    (set `self.Aperto` false :!label _label)
    (bind _foundwidgets (`WidgetBlueprintLibrary.GetAllWidgetsOfClass` "/Game/HUD/WidgetHUDGiocatore/BPWIdgetCassa.BPWIdgetCassa_C"))
    (for _array_element _foundwidgets
      (`Widget.RemoveFromParent` _array_element)
      (bind _foundwidgets_2 (`WidgetBlueprintLibrary.GetAllWidgetsOfClass` "/Game/HUD/WIdgetOggetti/BPWidgetObjSelezionato.BPWidgetObjSelezionato_C"))
      (for _array_element_2 _foundwidgets_2
        (if (`|EnumEquality` (`/Game/HUD/WIdgetOggetti/BPWidgetObjSelezionato.Provenienza` _array_element_2) "NewEnumerator9")
          (`Widget.RemoveFromParent` _array_element_2))))
    (else
      (bind _returnvalue (`|CreateWidget` "/Game/HUD/WidgetHUDGiocatore/BPWIdgetCassa.BPWIdgetCassa_C" null (`self.Drop`) self))
      (`UserWidget.AddToViewport` _returnvalue 0)
      (set `self.Aperto` true))))

(event `/Game/Blueprint/BPInterface.StopInteragisci`
  (goto _label))

(event `/Game/Blueprint/BPInterface.AttivaTesto`
  (`SceneComponent.SetVisibility` (`self.Testo`) true false))

(event `/Game/Blueprint/BPInterface.DisattivaTesto`
  (`SceneComponent.SetVisibility` (`self.Testo`) false false :!label _label_2))

(event `self.ReceiveBeginPlay`
  (goto _label_2))

(fn `UserConstructionScript`)