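; Turn-based battle manager that moves the player and an enemy into an arena, runs their fight and restores exploration afterwards.
; BattleMode plays a material-wipe transition, teleports both to marker actors and switches the camera to itself.
; Attacca alternates turns through the HUD, using timeline lerps and animation-length delays before applying damage.
; Either side reaching zero health calls NormalMode(true), which destroys the enemy and spawns a loot chest.
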(event `self.ReceiveBeginPlay`
  (bind (_effettitransizionest_distorsione _effettitransizionest_triangoli _effettitransizionest_strisce) (break `/Game/Grafica/Transizioni/EffettiTransizioneST` (`self.EffettiTransizioneST`)))
  ;[1 1 1] Inizializzazione variabili
  (bind _asbppersonaggio (cast `/Game/Blueprint/BPPersonaggio` (`GameplayStatics.GetPlayerCharacter` 0)))
  (set `self.Giocatore` _asbppersonaggio)
  (bind _outactors (`GameplayStatics.GetAllActorsOfClass` "/Game/Blueprint/BPAvversario.BPAvversario_C"))
  (for _array_element _outactors
    (set `/Game/Blueprint/BPAvversario.GestBattaglia` self _array_element)
    (bind _returnvalue (`|CreateWidget` "/Game/HUD/BPWidgetTransizione.BPWidgetTransizione_C"))
    (bind _output_get (set `self.WidgetTransizione` _returnvalue))
    (`Image.SetBrushFromMaterial` (`/Game/HUD/BPWidgetTransizione.ImmagineTransizione` _output_get) (select `/Game/Grafica/Transizioni/EffettiTransizioniEN` (`self.EffettiTransizioneEN`) :`NewEnumerator0` _effettitransizionest_triangoli :`NewEnumerator1` _effettitransizionest_strisce :`NewEnumerator2` _effettitransizionest_distorsione))))

(event `BattleMode`
  (params (Nemico :type "/Game/Blueprint/BPAvversario Object Reference") (Effetto :type "/Game/Grafica/Transizioni/EffettiTransizioniEN Enum" :default "NewEnumerator0"))
  (bind _widgettransizione (`self.WidgetTransizione`))
  (bind _giocatore (`self.Giocatore`))
  (bind _materialetransizione (`/Game/HUD/BPWidgetTransizione.MaterialeTransizione` _widgettransizione))
  ;[1 1 1] Inizia il combattimento
  (bind _output_get (set `self.Nemico` Nemico))
  (set `/Game/Blueprint/BPAvversario.SkillNemicoEN` "NewEnumerator3" _output_get)
  (bind _asbppersonaggio (cast `/Game/Blueprint/BPPersonaggio` (`GameplayStatics.GetPlayerCharacter` 0)))
  (`CharacterMovementComponent.DisableMovement` (`Character.CharacterMovement` _asbppersonaggio))
  (`CharacterMovementComponent.DisableMovement` (`Character.CharacterMovement` _output_get))
  (`self.DisableInput` _asbppersonaggio null)
  (set `PlayerController.bShowMouseCursor` true (`GameplayStatics.GetPlayerController` 0))
  (set `/Game/Blueprint/BPPersonaggio.MossaScelta` "NewEnumerator6" _giocatore)
  (set `self.PosizioneDrop` (`SceneComponent.K2_GetComponentToWorld` (`Actor.RootComponent` (`self.Nemico`))))
  (set `self.PosizioneGiocatore` (`SceneComponent.K2_GetComponentToWorld` (`Actor.RootComponent` _giocatore)))
  (`UserWidget.AddToViewport` _widgettransizione 0)
  (bind (_direction _newtrack_0) (`Timeline|Timeline_4` :!via `PlayFromStart`)
    (:`Update`
      (`MaterialInstanceDynamic.SetScalarParameterValue` _materialetransizione "Alpha" _newtrack_0))
    (:`Finished`
      (`self.SetUpBattaglia`)
      (bind (_direction_2 _newtrack_0_2) (`Timeline|Timeline_5` :!via `PlayFromStart`)
        (:`Update`
          (`MaterialInstanceDynamic.SetScalarParameterValue` _materialetransizione "Alpha" _newtrack_0_2))
        (:`Finished`
          (`self.Turno Giocatore`)
          (`Widget.SetVisibility` _widgettransizione "Visible"))))))

(event `SetUpBattaglia`
  ;[1 1 1] Preparazione alla battaglia
  (`PlayerController.SetViewTargetWithBlend` (`GameplayStatics.GetPlayerController` 0) self 0.0 "VTBlend_Linear" 0.0 false)
  (`SceneComponent.K2_SetWorldLocation` (`Actor.RootComponent` (`self.Giocatore`)) (`SceneComponent.K2_GetComponentLocation` (`Actor.RootComponent` (`self.PosGiocatore`))) false true)
  (`SceneComponent.K2_SetWorldLocation` (`Actor.RootComponent` (`self.Nemico`)) (`SceneComponent.K2_GetComponentLocation` (`Actor.RootComponent` (`self.PosNemico`))) false true)
  (bind _outactors (`GameplayStatics.GetAllActorsOfClass` "/Game/Blueprint/BPAvversario.BPAvversario_C"))
  (for _array_element _outactors
    (`CharacterMovementComponent.DisableMovement` (`Character.CharacterMovement` _array_element))))

(event `Turno Giocatore`
  ;[1 1 1] Passaggio turno
  (bind _asbphud (cast `/Game/HUD/BPHud` (`PlayerController.GetHUD` (`GameplayStatics.GetPlayerController` 0))))
  (`/Game/HUD/BPHud.HudTurnoGiocatore` _asbphud))

(event `Turno Avversario`
  ;[1 1 1] Passaggio turno
  (`/Game/HUD/BPHud.HudTurnoNemico` (stale `Turno Giocatore` _asbphud)))

(event `Attacca`
  (params (ChiAttacca :type "PaperCharacter Object Reference") (Danno :type Integer) (Mossa :type "/Game/Dati/Giocatore/DatiGiocatore1/MosseGiocatoreEN Enum" :default "NewEnumerator6"))
  (bind _returnvalue (* Danno -1))
  (bind _nemico (`self.Nemico`))
  (bind _giocatore (`self.Giocatore`))
  (bind _giocatore_2 (`self.Giocatore`))
  (bind _nemico_2 (`self.Nemico`))
  (bind _nemico_3 (`self.Nemico`))
  (bind _giocatore_3 (`self.Giocatore`))
  (bind _skillgiocatore (`/Game/Blueprint/BPPersonaggio.SkillGiocatore` (`self.Giocatore`)))
  (bind (_skillnemicost_idle _skillnemicost_posizioneattacco _skillnemicost_posizionenormale _skillnemicost_skill1) (break `/Game/Dati/Nemici/DatiNemici/MosseNemicoST` (`/Game/Blueprint/BPAvversario.SkillNemicoST` _nemico)))
  ;[1 1 1] Attacco del personaggio con scelta della mossa da fare, attacco del nemico
  (set `self.MossaGiocatore` Mossa)
  (cast `/Game/Blueprint/BPPersonaggio` ChiAttacca
    (:`then`
      (bind _foundwidgets (`WidgetBlueprintLibrary.GetAllWidgetsOfClass` "/Game/HUD/WidgetCombattimento/BPWidgetTurnoGiocatore.BPWidgetTurnoGiocatore_C"))
      (for _array_element _foundwidgets
        (`Widget.RemoveFromParent` _array_element))
      (set `/Game/Blueprint/BPPersonaggio.InBattaglia` true _giocatore)
      (set `/Game/Blueprint/BPPersonaggio.MossaScelta` "NewEnumerator3" _giocatore)
      (bind (_direction _newtrack_5) (`Timeline|Timeline_1` :!via `PlayFromStart`)
        (:`Update`
          (`self.MuoviInPosizione` _newtrack_5 (`self.PosGiocatore`) (`self.PosAttaccoGiocatore`) _giocatore_3))
        (:`Finished`
          (set `/Game/Blueprint/BPPersonaggio.MossaScelta` (`self.MossaGiocatore`) _giocatore_3)
          (`KismetSystemLibrary.Delay` (`PaperFlipbook.GetTotalDuration` (select `/Game/Dati/Giocatore/DatiGiocatore1/MosseGiocatoreEN` (`self.MossaGiocatore`) :`NewEnumerator3` (`.Animazione_6_A2D9DE42406F882B081E8284B2054071` (break `/Game/Dati/Giocatore/DatiGiocatore1/MossaGiocatore` (`.PosizioneAttacco_33_99F72B3E42193DE5B7E00B913B698B5E` (break `/Game/Dati/Giocatore/DatiGiocatore1/MosseAttualiGiocatoreST` _skillgiocatore)))) :`NewEnumerator4` (`.Animazione_6_A2D9DE42406F882B081E8284B2054071` (break `/Game/Dati/Giocatore/DatiGiocatore1/MossaGiocatore` (`.PosizioneDifesa_34_D2FF22644A8F68D2D9811B8363D5FD5A` (break `/Game/Dati/Giocatore/DatiGiocatore1/MosseAttualiGiocatoreST` _skillgiocatore)))) :`NewEnumerator5` (`.Animazione_6_A2D9DE42406F882B081E8284B2054071` (break `/Game/Dati/Giocatore/DatiGiocatore1/MossaGiocatore` (`.AttaccoBase_35_7EA19321457B0FFDB2FA7F97ED10EF87` (break `/Game/Dati/Giocatore/DatiGiocatore1/MosseAttualiGiocatoreST` _skillgiocatore)))) :`NewEnumerator0` (`.Animazione_6_A2D9DE42406F882B081E8284B2054071` (break `/Game/Dati/Giocatore/DatiGiocatore1/MossaGiocatore` (`.SkillSlot1_23_FCAA49F04AA8105ED0B0FC959EB98725` (break `/Game/Dati/Giocatore/DatiGiocatore1/MosseAttualiGiocatoreST` _skillgiocatore)))) :`NewEnumerator1` (`.Animazione_6_A2D9DE42406F882B081E8284B2054071` (break `/Game/Dati/Giocatore/DatiGiocatore1/MossaGiocatore` (`.SkillSlot2_24_7C31ACA9462EC4BBFBD063AD9AE19358` (break `/Game/Dati/Giocatore/DatiGiocatore1/MosseAttualiGiocatoreST` _skillgiocatore)))) :`NewEnumerator2` (`.Animazione_6_A2D9DE42406F882B081E8284B2054071` (break `/Game/Dati/Giocatore/DatiGiocatore1/MossaGiocatore` (`.SkillSlot3_25_90B495E643884197A2E6CBB1100D88DA` (break `/Game/Dati/Giocatore/DatiGiocatore1/MosseAttualiGiocatoreST` _skillgiocatore)))))))
          (`/Game/Blueprint/BPAvversario.AggiornaVita` (`self.Nemico`) _returnvalue)
          (set `/Game/Blueprint/BPPersonaggio.MossaScelta` "NewEnumerator4" _giocatore_3)
          (bind (_direction_2 _newtrack_5_2) (`Timeline|Timeline_0` :!via `PlayFromStart`)
            (:`Update`
              (`self.MuoviInPosizione` _newtrack_5_2 (`self.PosAttaccoGiocatore`) (`self.PosGiocatore`) _giocatore_2))
            (:`Finished`
              (set `/Game/Blueprint/BPPersonaggio.InBattaglia` true _giocatore_2)
              (if (<= (`/Game/Blueprint/BPAvversario.Vita` _nemico_2) 0)
                (`self.NormalMode` true :!label _label)
                (else
                  (`self.Turno Avversario`)
                  (set `/Game/Blueprint/BPPersonaggio.MossaScelta` "NewEnumerator6" _giocatore_2))))))))
    (:`CastFailed`
      (cast `/Game/Blueprint/BPAvversario` ChiAttacca)
      (set `/Game/Blueprint/BPAvversario.InBattaglia` true _nemico)
      (set `/Game/Blueprint/BPAvversario.SkillNemicoEN` "NewEnumerator0" _nemico)
      (bind (_direction_3 _newtrack_5_3) (`Timeline|Timeline_2` :!via `PlayFromStart`)
        (:`Update`
          (`self.MuoviInPosizione` _newtrack_5_3 (`self.PosNemico`) (`self.PosAttaccoNemico`) _nemico_3))
        (:`Finished`
          (set `/Game/Blueprint/BPAvversario.SkillNemicoEN` "NewEnumerator2" _nemico_3)
          (`KismetSystemLibrary.Delay` (`PaperFlipbook.GetTotalDuration` _skillnemicost_skill1))
          (`/Game/Blueprint/BPPersonaggio.AggiornaVita` (`self.Giocatore`) _returnvalue)
          (set `/Game/Blueprint/BPAvversario.SkillNemicoEN` "NewEnumerator1" _nemico_3)
          (bind (_direction_4 _newtrack_5_4) (`Timeline|Timeline_3` :!via `PlayFromStart`)
            (:`Update`
              (`self.MuoviInPosizione` _newtrack_5_4 (`self.PosAttaccoNemico`) (`self.PosNemico`) _nemico_2))
            (:`Finished`
              (set `/Game/Blueprint/BPAvversario.InBattaglia` true _nemico_2)
              (if (<= (`/Game/Blueprint/BPPersonaggio.VIta` _giocatore_2) 0)
                (goto _label)
                (else
                  (bind _foundwidgets_2 (`WidgetBlueprintLibrary.GetAllWidgetsOfClass` "/Game/HUD/WidgetCombattimento/BPWidgetTurnoAvversario.BPWidgetTurnoAvversario_C"))
                  (for _array_element_2 _foundwidgets_2
                    (`Widget.RemoveFromParent` _array_element_2))
                  (`self.Turno Giocatore`)
                  (set `/Game/Blueprint/BPAvversario.SkillNemicoEN` "NewEnumerator3" _nemico_2))))))))))

(event `NormalMode`
  (params (Esito :type Boolean))
  (bind _giocatore (`self.Giocatore`))
  (bind _nemico (`self.Nemico`))
  (bind _posizionedrop_location (`KismetMathLibrary.BreakTransform` (`self.PosizioneDrop`)))
  ;[1 1 1] Esito della partita con uscita dal combattimento
  (if Esito
    (set `self.DropNemico` (`/Game/Blueprint/BPAvversario.Drop` _nemico))
    (`self.K2_DestroyActor` _nemico)
    (bind _asbppersonaggio (cast `/Game/Blueprint/BPPersonaggio` (`GameplayStatics.GetPlayerCharacter` 0)))
    (`self.EnableInput` _asbppersonaggio null)
    (`SceneComponent.K2_SetWorldTransform` (`Actor.RootComponent` _giocatore) (`self.PosizioneGiocatore`) false true)
    (`CharacterMovementComponent.SetMovementMode` (`Character.CharacterMovement` _asbppersonaggio) "MOVE_Flying" 0)
    (set `PlayerController.bShowMouseCursor` false (`GameplayStatics.GetPlayerController` 0))
    (`PlayerController.SetViewTargetWithBlend` (`GameplayStatics.GetPlayerController` 0) (`GameplayStatics.GetPlayerCharacter` 0) 0.0 "VTBlend_Linear" 0.0 false)
    (bind _asbphud (cast `/Game/HUD/BPHud` (`PlayerController.GetHUD` (`GameplayStatics.GetPlayerController` 0))))
    (`/Game/HUD/BPHud.HudNormale` _asbphud)
    (bind _outactors (`GameplayStatics.GetAllActorsOfClass` "/Game/Blueprint/BPAvversario.BPAvversario_C"))
    (for _array_element _outactors
      (`CharacterMovementComponent.SetMovementMode` (`Character.CharacterMovement` _array_element) "MOVE_Flying" 0)
      (set `/Game/Blueprint/BPAvversario.staInteragendo` false _array_element))
    (set `/Game/Blueprint/BPPersonaggio.InBattaglia` false _giocatore)
    (`|SpawnActorFromClass` "/Game/Blueprint/Combattimento/BPCassa.BPCassa_C" (`KismetMathLibrary.MakeTransform` _posizionedrop_location) "AdjustIfPossibleButDontSpawnIfColliding" "OverrideRootScale" null (`self.DropNemico`) null)))

(fn `MuoviInPosizione`
  (params (Lerp :type "Float (double-precision)") (PosizioneIniziale :type "Actor Object Reference") (PosizioneFinale :type "Actor Object Reference") (ChiDevoSpostare :type "PaperCharacter Object Reference"))
  (`self.K2_SetActorRelativeLocation` ChiDevoSpostare (`KismetMathLibrary.VLerp` (`self.K2_GetActorLocation` PosizioneIniziale) (`self.K2_GetActorLocation` PosizioneFinale) Lerp) false false))

(fn `UserConstructionScript`)