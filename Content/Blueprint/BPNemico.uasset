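; BPNemico is an enemy character that drives a directional flipbook sprite every tick through GestoreAnimazioni.
; UltimaDirezione sets the Box's yaw and selects a movement or idle flipbook from AnimazioniPersonaggio based on speed, with climbing directions using the same clips for both.
; The velocity-based direction update sits behind an always-false constant comparison, so it never runs.
; The closing CollisioneFrontale validity check triggers nothing.
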(event `self.ReceiveTick`
  (params (DeltaSeconds :type "Float (single-precision)"))
  (`self.GestoreAnimazioni`))

(fn `GestoreAnimazioni`
  (bind (_animazionipersonaggio_muovisu _animazionipersonaggio_idlesu _animazionipersonaggio_muovigiu _animazionipersonaggio_idlegiu _animazionipersonaggio_muovisinistra _animazionipersonaggio_idlesinistra _animazionipersonaggio_muovidestra _animazionipersonaggio_idledestra _animazionipersonaggio_scalasu _animazionipersonaggio_scalagiu) (break `/Game/Dati/MovimentoGiocatoreST` (`self.AnimazioniPersonaggio`)))
  (bind _ultimadirezione (`self.UltimaDirezione`))
  (bind (_velocity_x _velocity_y _velocity_z) (`KismetMathLibrary.BreakVector` (`MovementComponent.Velocity` (`self.CharacterMovement`))))
  (if (or (!= 0.0 0.0) (!= 0.0 0.0))
    (if (> _velocity_x 0.0)
      (set `self.UltimaDirezione` "NewEnumerator0")
      (elif (< _velocity_x 0.0)
        (set `self.UltimaDirezione` "NewEnumerator1")
        (elif (> _velocity_z 0.0)
          (set `self.UltimaDirezione` "NewEnumerator3")
          (elif (< _velocity_z 0.0)
            (set `self.UltimaDirezione` "NewEnumerator2"))))))
  (`SceneComponent.K2_SetRelativeRotation` (`self.Box`) (select `/Game/Dati/MovimentoGiocatoreEN` (`self.UltimaDirezione`) :`NewEnumerator1` (struct :`Pitch` 180.0) :`NewEnumerator2` (struct :`Pitch` 90.0) :`NewEnumerator3` (struct :`Pitch` 270.0) :`NewEnumerator5` (struct :`Pitch` 180.0) :!type "Rotator Structure") false false)
  (`PaperFlipbookComponent.SetFlipbook` (`self.Sprite`) (select `bool` (> (`KismetMathLibrary.VSize` (`self.GetVelocity`)) 0.0) :`false` (select `/Game/Dati/MovimentoGiocatoreEN` _ultimadirezione :`NewEnumerator0` _animazionipersonaggio_idlesu :`NewEnumerator1` _animazionipersonaggio_idlegiu :`NewEnumerator2` _animazionipersonaggio_idlesinistra :`NewEnumerator3` _animazionipersonaggio_idledestra :`NewEnumerator4` _animazionipersonaggio_scalasu :`NewEnumerator5` _animazionipersonaggio_scalagiu) :`true` (select `/Game/Dati/MovimentoGiocatoreEN` _ultimadirezione :`NewEnumerator0` _animazionipersonaggio_muovisu :`NewEnumerator1` _animazionipersonaggio_muovigiu :`NewEnumerator2` _animazionipersonaggio_muovisinistra :`NewEnumerator3` _animazionipersonaggio_muovidestra :`NewEnumerator4` _animazionipersonaggio_scalasu :`NewEnumerator5` _animazionipersonaggio_scalagiu)))
  (if (`KismetSystemLibrary.IsValid` (`self.CollisioneFrontale`))
    _))

(fn `UserConstructionScript`)