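; Paper2D enemy that chases the player and starts a battle on contact.
; RicercaGiocatore overlap records the current position and starts an AI chase without pathfinding, then sends it back on exit; CollisioneFrontale hands it to GestBattaglia.
; TipoNemico selects movement and skill data; GestoreAnimazioni picks flipbooks every tick from velocity or battle skill state, rotating Box with facing.
; Custom events update health and save or restore its transform.
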(event `self.ReceiveBeginPlay`
  (bind (_tiponemicost_nemico1 _tiponemicost_nemico2 _tiponemicost_nemico3) (break `/Game/Dati/Nemici/TIpoNemicoST` (`self.TipoNemicoST`)))
  (bind (_returnvalue_filemovimentonemico _returnvalue_movimentipossibilinemico _returnvalue_filemossenemico _returnvalue_mossepossibilinemico) (break `/Game/Dati/Nemici/DatiNemici/DatiNemicoST` (select `/Game/Dati/Nemici/TIpoNemicoEN` (`self.TipoNemico`) :`NewEnumerator0` _tiponemicost_nemico1 :`NewEnumerator1` _tiponemicost_nemico2 :`NewEnumerator2` _tiponemicost_nemico3)))
  (set `self.AnimazioniPersonaggio` _returnvalue_filemovimentonemico)
  (set `self.UltimaDirezione` _returnvalue_movimentipossibilinemico)
  (set `self.SkillNemicoST` _returnvalue_filemossenemico)
  (set `self.SkillNemicoEN` _returnvalue_mossepossibilinemico))

(event `self.ReceiveTick`
  (params (DeltaSeconds :type "Float (single-precision)"))
  (`self.GestoreAnimazioni`))

(event `self.CollisioneFrontale.OnComponentBeginOverlap`
  (params (OverlappedComponent :type "PrimitiveComponent Object Reference") (OtherActor :type "Actor Object Reference") (OtherComp :type "PrimitiveComponent Object Reference") (OtherBodyIndex :type Integer) (bFromSweep :type Boolean) (SweepResult :type "HitResult Structure (by ref)"))
  (bind _gestbattaglia (`self.GestBattaglia`))
  ;[1 1 1] Inizio battaglia quando il giocatore è abbastanza vicino
  (if (not (`self.staInteragendo`))
    (cast `/Game/Blueprint/BPPersonaggio` OtherActor)
    (`/Engine/EditorBlueprintResources/StandardMacros.IsValid` _gestbattaglia
      (:`Is Valid`
        (`/Game/Blueprint/ManagerBattaglia.BattleMode` _gestbattaglia self)
        (set `self.staInteragendo` true)
        (`Controller.StopMovement` (`AIBlueprintHelperLibrary.GetAIController` self))))))

(event `AggiornaVita`
  (params (Vita :type Integer))
  ;[1 1 1] Aggiornamento vita
  (set `self.VIta` (+ Vita (`self.VIta`))))

(event `Carica Posizione`
  ;[1 1 1] Salvataggio e caricamento
  (bind _returnvalue (`GameplayStatics.DoesSaveGameExist` (`self.SaveSlot`)))
  (if _returnvalue
    (bind _returnvalue_2 (`GameplayStatics.LoadGameFromSlot` (`self.SaveSlot`)))
    (bind _output_get (set `self.SaverSubclass` _returnvalue_2))
    (bind _asbpsalva_gioco (cast `/Game/Blueprint/BPSalvaGioco` _output_get))
    (`self.K2_SetActorTransform` (`/Game/Blueprint/BPSalvaGioco.Posizione` _asbpsalva_gioco))
    (else
      (bind _returnvalue_3 (`GameplayStatics.CreateSaveGameObject` "/Game/Blueprint/BPSalvaGioco.BPSalvaGioco_C" :!label _label))
      (bind _output_get_2 (set `self.SaverSubclass` _returnvalue_3))
      (bind _asbpsalva_gioco_2 (cast `/Game/Blueprint/BPSalvaGioco` _output_get_2))
      (set `/Game/Blueprint/BPSalvaGioco.Posizione` (`self.GetTransform`) _asbpsalva_gioco_2)
      (set `/Game/Blueprint/BPSalvaGioco.Direzione` "NewEnumerator0" _asbpsalva_gioco_2)
      (`GameplayStatics.SaveGameToSlot` (`self.SaverSubclass`) (`self.SaveSlot`))
      (`KismetSystemLibrary.PrintString` (`KismetStringLibrary.Conv_TransformToString` (`self.GetTransform`)) true true (struct :`R` 1.0 :`G` 0.035682 :`A` 1.0)))))

(event `Salva Posizione`
  ;[1 1 1] Salvataggio e caricamento
  (goto _label))

(event `self.RicercaGiocatore.OnComponentBeginOverlap`
  (params (OverlappedComponent :type "PrimitiveComponent Object Reference") (OtherActor :type "Actor Object Reference") (OtherComp :type "PrimitiveComponent Object Reference") (OtherBodyIndex :type Integer) (bFromSweep :type Boolean) (SweepResult :type "HitResult Structure (by ref)"))
  (bind _returnvalue (`AIBlueprintHelperLibrary.GetAIController` self))
  ;[1 1 1] Inseguimento del giocatore
  (if (not (`self.InBattaglia`))
    (bind _asbppersonaggio (cast `/Game/Blueprint/BPPersonaggio` OtherActor))
    (set `self.PosizioneIniziale` (`KismetMathLibrary.MakeTransform` (`self.K2_GetActorLocation` self)))
    (`Controller.StopMovement` _returnvalue)
    (`AITask_MoveTo.AIMoveTo` _returnvalue (`self.K2_GetActorLocation` _asbppersonaggio) _asbppersonaggio -1.0 "Default" "Default" false)))

(event `self.RicercaGiocatore.OnComponentEndOverlap`
  (params (OverlappedComponent :type "PrimitiveComponent Object Reference") (OtherActor :type "Actor Object Reference") (OtherComp :type "PrimitiveComponent Object Reference") (OtherBodyIndex :type Integer))
  (bind _posizioneiniziale_location (`KismetMathLibrary.BreakTransform` (`self.PosizioneIniziale`)))
  (bind _returnvalue (`AIBlueprintHelperLibrary.GetAIController` self))
  ;[1 1 1] Quando il giocatore si è allontanato troppo, ritorna alla posizione iniziale
  (cast `/Game/Blueprint/BPPersonaggio` OtherActor)
  (`Controller.StopMovement` _returnvalue)
  (`AIController.MoveToLocation` _returnvalue _posizioneiniziale_location -1.0 true false false true null true))

(fn `GestoreAnimazioni`
  (bind (_returnvalue_x _returnvalue_y _returnvalue_z) (`KismetMathLibrary.BreakVector` (`self.GetVelocity`)))
  (bind (_returnvalue_x_2 _returnvalue_y_2 _returnvalue_z_2) (`KismetMathLibrary.BreakVector` (`self.GetVelocity`)))
  (bind (_animazionipersonaggio_muovisu _animazionipersonaggio_idlesu _animazionipersonaggio_muovigiu _animazionipersonaggio_idlegiu _animazionipersonaggio_muovisinistra _animazionipersonaggio_idlesinistra _animazionipersonaggio_muovidestra _animazionipersonaggio_idledestra _animazionipersonaggio_scalasu _animazionipersonaggio_scalagiu) (break `/Game/Dati/Nemici/DatiNemici/AnimazioniNemicoST` (`self.AnimazioniPersonaggio`)))
  (bind (_skillnemicost_posizioneattacco _skillnemicost_posizionenormale _skillnemicost_skill1) (break `/Game/Dati/Nemici/DatiNemici/MosseNemicoST` (`self.SkillNemicoST`)))
  (bind _ultimadirezione (`self.UltimaDirezione`))
  (if (`self.InBattaglia`)
    (`PaperFlipbookComponent.SetFlipbook` (`self.Sprite`) (select `/Game/Dati/Nemici/DatiNemici/MosseNemicoEN` (`self.SkillNemicoEN`) :`NewEnumerator0` _skillnemicost_posizioneattacco :`NewEnumerator1` _skillnemicost_posizionenormale :`NewEnumerator2` _skillnemicost_skill1))
    (else
      (if (or (!= _returnvalue_x 0.0) (!= _returnvalue_z 0.0))
        (if (> _returnvalue_z_2 60.0)
          (set `self.UltimaDirezione` "NewEnumerator0")
          (elif (< _returnvalue_z_2 -60.0)
            (set `self.UltimaDirezione` "NewEnumerator1")
            (elif (> _returnvalue_x_2 0.0)
              (set `self.UltimaDirezione` "NewEnumerator3")
              (elif (< _returnvalue_x_2 0.0)
                (set `self.UltimaDirezione` "NewEnumerator3"))))))
      (`SceneComponent.K2_SetRelativeRotation` (`self.Box`) (select `/Game/Dati/Nemici/DatiNemici/AnimazioniNemicoEN` (`self.UltimaDirezione`) :`NewEnumerator1` (struct :`Pitch` 180.0) :`NewEnumerator2` (struct :`Pitch` 90.0) :`NewEnumerator3` (struct :`Pitch` 270.0) :`NewEnumerator5` (struct :`Pitch` 180.0) :!type "Rotator Structure") false false)
      (`PaperFlipbookComponent.SetFlipbook` (`self.Sprite`) (select `bool` (> (`KismetMathLibrary.VSize` (`self.GetVelocity`)) 0.0) :`false` (select `/Game/Dati/Nemici/DatiNemici/AnimazioniNemicoEN` _ultimadirezione :`NewEnumerator0` _animazionipersonaggio_idlesu :`NewEnumerator1` _animazionipersonaggio_idlegiu :`NewEnumerator2` _animazionipersonaggio_idlesinistra :`NewEnumerator3` _animazionipersonaggio_idledestra :`NewEnumerator4` _animazionipersonaggio_scalasu :`NewEnumerator5` _animazionipersonaggio_scalagiu) :`true` (select `/Game/Dati/Nemici/DatiNemici/AnimazioniNemicoEN` _ultimadirezione :`NewEnumerator0` _animazionipersonaggio_muovisu :`NewEnumerator1` _animazionipersonaggio_muovigiu :`NewEnumerator2` _animazionipersonaggio_muovisinistra :`NewEnumerator3` _animazionipersonaggio_muovidestra :`NewEnumerator4` _animazionipersonaggio_scalasu :`NewEnumerator5` _animazionipersonaggio_scalagiu))))))

(fn `UserConstructionScript`)