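; Sound manager Blueprint that handles ambient music, battle music and one-shot effects.
; BeginPlay spawns the ambient track; PlayBattaglia pauses it and spawns combat music, while PlayNormale stops combat and resumes ambient.
; Play events fire 2D one-shots at ambient or effect volume, with PlayAmbient also stopping combat music.
; Pause and normal events switch music volume, but Tick reapplies normal ambient volume every frame, overriding the pause level.
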(event `self.ReceiveTick`
  (params (DeltaSeconds :type "Float (single-precision)"))
  (bind _localmusicacombattimento (`self.LocalMusicaCombattimento`))
  (`AudioComponent.SetVolumeMultiplier` (`self.LocalMusicaAmbient`) (`self.VolumeAmbient`))
  (`/Engine/EditorBlueprintResources/StandardMacros.IsValid` _localmusicacombattimento
    (:`Is Valid`
      (`AudioComponent.SetVolumeMultiplier` _localmusicacombattimento (`self.VolumeAmbient`)))))

(event `self.ReceiveBeginPlay`
  (bind _returnvalue (`GameplayStatics.SpawnSound2D` (`self.MusicaAmbientale`) (`self.VolumeAmbient`)))
  (set `self.LocalMusicaAmbient` _returnvalue))

(event `VolumePausa`
  (bind _localmusicacombattimento (`self.LocalMusicaCombattimento`))
  (`AudioComponent.SetVolumeMultiplier` (`self.LocalMusicaAmbient`) (`self.VolumeAmbientPausa`))
  (`/Engine/EditorBlueprintResources/StandardMacros.IsValid` _localmusicacombattimento
    (:`Is Valid`
      (`AudioComponent.SetVolumeMultiplier` _localmusicacombattimento (`self.VolumeAmbientPausa`)))))

(event `VolumeNormale`
  (bind _localmusicacombattimento (`self.LocalMusicaCombattimento`))
  (`AudioComponent.SetVolumeMultiplier` (`self.LocalMusicaAmbient`) (`self.VolumeAmbient`))
  (`/Engine/EditorBlueprintResources/StandardMacros.IsValid` _localmusicacombattimento
    (:`Is Valid`
      (`AudioComponent.SetVolumeMultiplier` _localmusicacombattimento (`self.VolumeAmbient`)))))

(event `PlayAmbient`
  (params (NewParam :type "SoundBase Object Reference"))
  (`GameplayStatics.PlaySound2D` NewParam (`self.VolumeAmbient`))
  (`AudioComponent.Stop` (`self.LocalMusicaCombattimento`)))

(event `PlayNormale`
  (`AudioComponent.SetPaused` (`self.LocalMusicaAmbient`) false)
  (`AudioComponent.Stop` (`self.LocalMusicaCombattimento`)))

(event `PlayBattaglia`
  (`AudioComponent.SetPaused` (`self.LocalMusicaAmbient`) true)
  (bind _returnvalue (`GameplayStatics.SpawnSound2D` (`self.MusicaCombattimento`) (`self.VolumeAmbient`)))
  (set `self.LocalMusicaCombattimento` _returnvalue))

(event `PlayEffect`
  (params (NewParam :type "SoundBase Object Reference"))
  (`GameplayStatics.PlaySound2D` NewParam (`self.VolumeEffect`)))

(fn `UserConstructionScript`)